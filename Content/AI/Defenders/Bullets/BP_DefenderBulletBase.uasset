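; Base projectile actor fired by AI defenders that damages enemies it touches.
; On BeginPlay it binds a handler to its actor overlap event and starts a short lifetime delay, after which it destroys itself.
; Overlapping a BP_BaseEnemy applies fixed damage with the bullet as causer, then destroys it immediately; other actors are ignored.
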(event Custom|CustomEvent
  (params (OverlappedActor :type Actor%20Object%20Reference) (OtherActor :type Actor%20Object%20Reference))
  (bind _asbp_base_enemy (Utilities|Casting|CastToBP_BaseEnemy OtherActor))
  (Game|Damage|ApplyDamage _asbp_base_enemy 5e+01 0 self "/Script/Engine.DamageType")
  (Actor|DestroyActor))

(event EventBeginPlay
  (|CallParentFunction)
  (EventDispatchers|BindEventtoOnActorBeginOverlap (delegate Custom|CustomEvent))
  (Utilities|FlowControl|Delay 5.0)
  (Actor|DestroyActor))

(event Collision|EventActorBeginOverlap
  (params (OtherActor :type Actor%20Object%20Reference))
  (|CallParentFunction OtherActor) ; This node is disabled and will not be called.\nDrag off pins to build functionality.
)

(event EventTick
  (params (DeltaSeconds :type Float%20%28single-precision%29))
  (|CallParentFunction DeltaSeconds) ; This node is disabled and will not be called.\nDrag off pins to build functionality.
)

(fn ConstructionScript
  (|CallParentFunction))