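; BP_MeleeAttack is a short-lived AI melee hit actor that damages defenders through a sphere overlap.
; Init stores the damage amount supplied from outside.
; When the sphere overlaps a BP_DefenderBase, it spawns attached sparks, applies that damage and destroys itself after a brief delay.
; Any other overlap only starts a longer delayed destroy, and nothing here removes the actor without an overlap.
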(event OnComponentBeginOverlap(Sphere)
  (params (OverlappedComponent :type Primitive%20Component%20Object%20Reference) (OtherActor :type Actor%20Object%20Reference) (OtherComp :type Primitive%20Component%20Object%20Reference) (OtherBodyIndex :type Integer) (bFromSweep :type Boolean) (SweepResult :type Hit%20Result%20Structure%20%28by%20ref%29))
  (bind _asbp_defender_base (Utilities|Casting|CastToBP_DefenderBase OtherActor)
    (:then
      (Effects|SpawnEmitterAttached "/Game/Realistic_Starter_VFX_Pack_Vol2/Particles/Sparks/P_Sparks_E.P_Sparks_E" (Variables|Default|GetDefaultSceneRoot) "None" (Transformation|GetActorLocation self) "0, 0, 0" "3.000000,3.000000,3.000000" "KeepWorldPosition")
      (Game|Damage|ApplyDamage _asbp_defender_base (Variables|Default|GetDamage) 0 self "/Script/Engine.DamageType")
      (Utilities|FlowControl|Delay 1.0)
      (Actor|DestroyActor))
    (:CastFailed
      (Utilities|FlowControl|Delay 2.0)
      (Actor|DestroyActor))))

(event EventBeginPlay)

(event Collision|EventActorBeginOverlap
  (params (OtherActor :type Actor%20Object%20Reference)))

(event EventTick
  (params (DeltaSeconds :type Float%20%28single-precision%29)))

(fn ConstructionScript)

(fn Init
  (params (Damage :type Float%20%28double-precision%29))
  (Variables|Default|SetDamage Damage))