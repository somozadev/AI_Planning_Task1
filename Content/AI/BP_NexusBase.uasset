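; BP_NexusBase is an AI defensive base actor with data-driven targeting and health, apparently a turret-style parent class.
; Targets are filtered by casting pawns to ground or air enemies per its anti-ground, anti-air or multi type.
; Helpers clear Blackboard target and sense keys, though ResetHeard writes TargetSeen instead of TargetHeard.
; Damaged subtracts health or explodes and destroys the actor, but AnyDamage and BeginPlay are empty, leaving it unwired here.
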(event EventBeginPlay)

(event Game|Damage|EventAnyDamage
  (params (Damage :type Float%20%28single-precision%29) (DamageType :type Damage%20Type%20Object%20Reference) (InstigatedBy :type Controller%20Object%20Reference) (DamageCauser :type Actor%20Object%20Reference)))

(fn ConstructionScript)

(fn ResetBlackboardValue
  (params (ResetActor :type Boolean) (ResetSeen :type Boolean) (ResetHeard :type Boolean))
  (Utilities|FlowControl|Sequence
    (:then_0
      (if ResetActor
        (AI|Components|Blackboard|SetValueasObject (Variables|Default|GetBlackboard) (Utilities|Name|MakeLiteralName "TargetActor") 0)))
    (:then_1
      (if ResetSeen
        (AI|Components|Blackboard|SetValueasBool (Variables|Default|GetBlackboard) (Utilities|Name|MakeLiteralName "TargetSeen") false)))
    (:then_2
      (if ResetHeard
        (AI|Components|Blackboard|SetValueasBool (Variables|Default|GetBlackboard) (Utilities|Name|MakeLiteralName "TargetSeen") false)))))

(fn UpdateCurrentStateDisplay
  (params (Text :type Text%20%28by%20ref%29)))

(fn CasttoEnemyTarget
  (params (Pawn :type Pawn%20Object%20Reference))
  (switch Utilities|FlowControl|Switch|SwitchonEnum_DefenderType (.type (Variables|Default|GetData))
    (:NewEnumerator0
      (bind _asbp_ground_enemy (Utilities|Casting|CastToBP_GroundEnemy Pawn)
        (:then
          (return _asbp_ground_enemy))
        (:CastFailed
          _)))
    (:NewEnumerator1
      (bind _asbp_air_enemy (Utilities|Casting|CastToBP_AirEnemy Pawn)
        (:then
          (return _asbp_air_enemy))
        (:CastFailed
          _)))
    (:NewEnumerator2
      (bind _asbp_ground_enemy_2 (Utilities|Casting|CastToBP_GroundEnemy Pawn)
        (:then
          (return _asbp_ground_enemy_2))
        (:CastFailed
          (bind _asbp_air_enemy_2 (Utilities|Casting|CastToBP_AirEnemy Pawn)
            (:then
              (return _asbp_air_enemy_2))
            (:CastFailed
              _))))))
  (return 0))

(fn CastFailedEnemyNotTargeteable
  (params (Sight :type Boolean))
  (bind _blackboard (Variables|Default|GetBlackboard))
  (AI|Components|Blackboard|SetValueasObject _blackboard (Utilities|Name|MakeLiteralName "TargetActor") 0)
  (if Sight
    (AI|Components|Blackboard|SetValueasBool _blackboard (Utilities|Name|MakeLiteralName "TargetSeen") false)
    (else
      (AI|Components|Blackboard|SetValueasBool _blackboard (Utilities|Name|MakeLiteralName "TargetHeard") false)))
  (return))

(fn Damaged
  (params (Damage :type Float%20%28double-precision%29))
  (if (>= Damage (.health (Variables|Default|GetData)))
    (Effects|SpawnEmitteratLocation "/Game/Realistic_Starter_VFX_Pack_Vol2/Particles/Explosion/P_Explosion_Big_B.P_Explosion_Big_B" (Transformation|GetActorLocation self) "0, 0, 0" "1.000000,1.000000,1.000000" true "AutoRelease")
    (Actor|DestroyActor)
    (else
      (Variables|Default|SetData (Utilities|Struct|MakeStruct_Defender (.type (Variables|Default|GetData)) (.targettype (Variables|Default|GetData)) (.preferredtypes (Variables|Default|GetData)) (.reloadtime (Variables|Default|GetData)) (.rotationspeed (Variables|Default|GetData)) (.sightangle (Variables|Default|GetData)) (.sightradius (Variables|Default|GetData)) (- (.health (Variables|Default|GetData)) Damage) (.damage (Variables|Default|GetData)))))))