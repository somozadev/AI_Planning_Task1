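; Base enemy pawn whose AI senses defenders and feeds its behavior tree blackboard.
; Sight, hearing and defender damage set target and stimulus keys, which retriggerable delays clear after a short lapse.
; It mirrors the game instance's current mode into the blackboard whenever that changes.
; A Data struct drives speed and health; lethal damage spawns an explosion, and destruction notifies the game instance.
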(event OnSeePawn(PawnSensing)
  (params (Pawn :type Pawn%20Object%20Reference))
  (bind _self self)
  (bind _returnvalue (AI|GetAIController _self))
  (bind _returnvalue_2 (AI|GetBlackboard _returnvalue))
  (bind _asbp_defender_base (Utilities|Casting|CastToBP_DefenderBase Pawn))
  (AI|Components|Blackboard|SetValueasObject _returnvalue_2 (Utilities|Name|MakeLiteralName "TargetActorRef") _asbp_defender_base)
  (AI|Components|Blackboard|SetValueasObject _returnvalue_2 (Utilities|Name|MakeLiteralName "LastTargetActorRef") _asbp_defender_base)
  (AI|Components|Blackboard|SetValueasBool _returnvalue_2 (Utilities|Name|MakeLiteralName "HasSeenTarget") true)
  (Utilities|FlowControl|RetriggerableDelay 2.0)
  (CallFunction|ResetBlackboardValue true true true false))

(event OnHearNoise(PawnSensing)
  (params (Instigator :type Pawn%20Object%20Reference) (Location :type Vector%20%28by%20ref%29 :default "0, 0, 0") (Volume :type Float%20%28single-precision%29))
  (bind _self self)
  (bind _returnvalue (AI|GetAIController _self))
  (bind _returnvalue_2 (AI|GetBlackboard _returnvalue))
  (bind _asbp_defender_base (Utilities|Casting|CastToBP_DefenderBase Instigator))
  (AI|Components|Blackboard|SetValueasObject _returnvalue_2 (Utilities|Name|MakeLiteralName "TargetActorRef") _asbp_defender_base)
  (AI|Components|Blackboard|SetValueasObject _returnvalue_2 (Utilities|Name|MakeLiteralName "LastTargetActorRef") _asbp_defender_base)
  (AI|Components|Blackboard|SetValueasBool _returnvalue_2 (Utilities|Name|MakeLiteralName "HasHeardTarget") true)
  (Utilities|FlowControl|RetriggerableDelay 2.0)
  (CallFunction|ResetBlackboardValue true true true false))

(event Custom|UpdateGameStateEnum
  (AI|Components|Blackboard|SetValueasEnum (AI|GetBlackboard (AI|GetAIController self)) (Utilities|Name|MakeLiteralName "CurrentPlanner") (Variables|/Game/MyGameInstance.MyGameInstance_C|GetCURRENT_GAMESTATE (stale EventBeginPlay _asmy_game_instance))))

(event EventBeginPlay
  (Variables|Default|SetBlackboard (AI|GetBlackboard (AI|GetAIController self)))
  (bind _asmy_game_instance (Utilities|Casting|CastToMyGameInstance (Game|GetGameInstance)))
  (EventDispatchers|BindEventtoOnModeChanged _asmy_game_instance (delegate Custom|UpdateGameStateEnum))
  (AI|Components|Blackboard|SetValueasEnum (AI|GetBlackboard (AI|GetAIController self)) (Utilities|Name|MakeLiteralName "CurrentPlanner") (Variables|/Game/MyGameInstance.MyGameInstance_C|GetCURRENT_GAMESTATE _asmy_game_instance)))

(event Collision|EventActorBeginOverlap
  (params (OtherActor :type Actor%20Object%20Reference)))

(event EventTick
  (params (DeltaSeconds :type Float%20%28single-precision%29)))

(event Game|Damage|EventAnyDamage
  (params (Damage :type Float%20%28single-precision%29) (DamageType :type Damage%20Type%20Object%20Reference) (InstigatedBy :type Controller%20Object%20Reference) (DamageCauser :type Actor%20Object%20Reference))
  (bind _self self)
  (bind _self_2 self)
  (bind _returnvalue (AI|GetAIController _self))
  (bind _returnvalue_2 (AI|GetAIController _self_2))
  (bind _returnvalue_3 (AI|GetBlackboard _returnvalue))
  (bind _returnvalue_4 (AI|GetBlackboard _returnvalue_2))
  (CallFunction|Damaged Damage)
  (Utilities|IsValid _returnvalue_3
    (:Is%20Valid
      (bind _asbp_defender_base (Utilities|Casting|CastToBP_DefenderBase DamageCauser))
      (AI|Components|Blackboard|SetValueasBool _returnvalue_3 (Utilities|Name|MakeLiteralName "DamageReceived") true)
      (AI|Components|Blackboard|SetValueasObject _returnvalue_4 (Utilities|Name|MakeLiteralName "LastTargetActorRef") _asbp_defender_base)
      (AI|Components|Blackboard|SetValueasObject _returnvalue_4 (Utilities|Name|MakeLiteralName "TargetActorRef") _asbp_defender_base)
      (Utilities|FlowControl|RetriggerableDelay 2.0)
      (CallFunction|ResetBlackboardValue false false false true))))

(event EventDestroyed
  (bind _asmy_game_instance (Utilities|Casting|CastToMyGameInstance (Game|GetGameInstance)))
  (Default|CallOnEnemyDeath _asmy_game_instance))

(fn ConstructionScript
  (bind _floatingpawnmovement (Variables|Default|GetFloatingPawnMovement))
  (Variables|/Script/Engine.FloatingPawnMovement|SetMaxSpeed _floatingpawnmovement (* (.Speed (Utilities|Struct|BreakSt_Enemy (Variables|Default|GetData))) (Class|MovementComponent|GetMaxSpeed _floatingpawnmovement))))

(fn Damaged
  (params (Damage :type Float%20%28double-precision%29))
  (if (>= Damage (.health (Variables|Default|GetData)))
    (Effects|SpawnEmitteratLocation "/Game/Realistic_Starter_VFX_Pack_Vol2/Particles/Explosion/P_Explosion_Big_B.P_Explosion_Big_B" (Transformation|GetActorLocation self) "0, 0, 0" "1.000000,1.000000,1.000000" true "AutoRelease")
    (Actor|DestroyActor)
    (else
      (Variables|Default|SetData (Utilities|Struct|MakeSt_Enemy (.type (Variables|Default|GetData)) (.targettype (Variables|Default|GetData)) (.preferredtypes (Variables|Default|GetData)) (- (.health (Variables|Default|GetData)) Damage) (.speed (Variables|Default|GetData)) (.attackrange (Variables|Default|GetData)) (.subtype (Variables|Default|GetData)) (.attackwaittime (Variables|Default|GetData)) (.damage (Variables|Default|GetData)))))))

(fn ResetBlackboardValue
  (params (ActorReset :type Boolean) (SeenReset :type Boolean) (HeardReset :type Boolean) (DamageReceivedCondition :type Boolean))
  (Utilities|FlowControl|Sequence
    (:then_0
      (if ActorReset
        (AI|Components|Blackboard|SetValueasObject (Variables|Default|GetBlackboard) (Utilities|Name|MakeLiteralName "TargetActorRef") 0)))
    (:then_1
      (if SeenReset
        (AI|Components|Blackboard|SetValueasBool (Variables|Default|GetBlackboard) (Utilities|Name|MakeLiteralName "HasSeenTarget") false)))
    (:then_2
      (if HeardReset
        (AI|Components|Blackboard|SetValueasBool (Variables|Default|GetBlackboard) (Utilities|Name|MakeLiteralName "HasHeardTarget") false)))
    (:then_3
      (if DamageReceivedCondition
        (AI|Components|Blackboard|SetValueasBool (Variables|Default|GetBlackboard) (Utilities|Name|MakeLiteralName "DamageReceived") false)))))

(fn EmitNoise
  (params (Loudness :type Float%20%28single-precision%29))
  (Class|PawnNoiseEmitterComponent|MakeNoise (Variables|Default|GetPawnNoiseEmitter) self Loudness (Transformation|GetActorLocation)))